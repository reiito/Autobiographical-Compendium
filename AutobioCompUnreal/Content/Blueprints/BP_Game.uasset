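; BP_Game is a game case on a shelf that pops in and out as selection moves between neighboring cases.
; BeginPlay sets up the PopInOut timeline, which slides the case between its start position and an offset.
; ShootTrace line-traces in a given direction for another BP_Game, reverses the BP_Shelf pawn's current game timeline, plays the neighbor's and returns it.
; A dynamic material instance lets SetNewProperties swap the cover texture alongside the name.
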(event `self.ReceiveBeginPlay`
  (`/Game/Blueprints/BP_Macros.SetupLerpTimeline` (`self.PopInOut`) "/Game/Data/CURVE_Linear.CURVE_Linear" "None" (`self.AnimationSpeed`)
    (:`__`
      (set `self.StartPos` (`SceneComponent.K2_GetComponentLocation` (`self.GameCase`))))))

(fn `SetNewProperties`
  (params (NewMaterial :type "Texture2D Object Reference") (Name :type String))
  (`MaterialInstanceDynamic.SetTextureParameterValue` (`self.MaterialInstance`) "Case" NewMaterial)
  (set `self.Name` Name))

(fn `ShootTrace`
  (params (Direction :type "/Game/Data/ENUM_Direction Enum" :default "NewEnumerator0"))
  (returns (NextObject :type "/Game/Blueprints/BP_Game Object Reference"))
  (bind _returnvalue (`SceneComponent.K2_GetComponentLocation` (`self.Base`)))
  (`|ExecutionSequence`
    (:`then_0`
      (switch `/Game/Data/ENUM_Direction` Direction
        (:`NewEnumerator0`
          (set `self.TraceDirection` (0.0 -1.0 0.0)))
        (:`NewEnumerator1`
          (set `self.TraceDirection` (0.0 1.0 0.0)))
        (:`NewEnumerator2`
          (set `self.TraceDirection` (0.0 0.0 1.0)))
        (:`NewEnumerator3`
          (set `self.TraceDirection` (0.0 0.0 -1.0)))))
    (:`then_1`
      (bind (_outhit _returnvalue_2) (`KismetSystemLibrary.LineTraceSingleForObjects` _returnvalue (+ _returnvalue (* (`self.TraceDirection`) (`self.TraceDistance`))) (`|MakeArray` "ObjectTypeQuery2" :!type "EObjectTypeQuery Enum")))
      (if _returnvalue_2
        (bind _asbp_game (cast `/Game/Blueprints/BP_Game` (`.HitActor` (`GameplayStatics.BreakHitResult` _outhit))))
        (bind _asbp_shelf (cast `/Game/Blueprints/BP_Shelf` (`GameplayStatics.GetPlayerPawn` 0)))
        (`TimelineComponent.Reverse` (`/Game/Blueprints/BP_Game.PopInOut` (`/Game/Blueprints/BP_Shelf.CurrentGame` _asbp_shelf)))
        (`TimelineComponent.Play` (`/Game/Blueprints/BP_Game.PopInOut` _asbp_game))
        (return _asbp_game)))))

(fn `UserConstructionScript`
  (bind _returnvalue (`KismetMaterialLibrary.CreateDynamicMaterialInstance` "/Game/Models/MAT_CD_Case_Inst.MAT_CD_Case_Inst"))
  (bind _output_get (set `self.MaterialInstance` _returnvalue))
  (`PrimitiveComponent.SetMaterial` (`self.GameCase`) 0 _output_get))