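; BP_Shelf is a game launcher shelf that lets the player browse BP_Game items and run the selected one as an executable.
; On begin play it gathers the games, assigns materials and names from YoungGames by index, and highlights the starting one.
; Directional inputs move the selection by tracing from the current game.
; Select disables input, opens the EXE through BP_ProcessTracker, then closes it after WeekTime and re-enables input.
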(event `self.ReceiveBeginPlay`
  (`self.GetProcessTracker`)
  (`self.GetGames`)
  (`self.InitGames`)
  (`TimelineComponent.Play` (`/Game/Blueprints/BP_Game.PopInOut` (`self.CurrentGame`))))

(event `Key|Escape`
  (params (Key :type "Key Structure"))
  (:`Pressed`
    (`KismetSystemLibrary.QuitGame` null "Quit")))

(event `InputAction|Select`
  (params (Key :type "Key Structure"))
  (bind _processtracker (`self.ProcessTracker`))
  (:`Pressed`
    (`self.DisableInput` null)
    (`ProcessManager.OpenEXE` (`/Game/Blueprints/BP_Game.Name` (`self.CurrentGame`)) _processtracker)
    (`KismetSystemLibrary.Delay` (`self.WeekTime`))
    (`ProcessManager.CloseEXE` _processtracker)
    (`self.EnableInput` null)))

(event `InputAction|Left`
  (params (Key :type "Key Structure"))
  (:`Pressed`
    (bind _running (`self.DirectionBehaviour` "NewEnumerator0"))
    (if _running
      (`KismetSystemLibrary.Delay` 0.2))))

(event `InputAction|Right`
  (params (Key :type "Key Structure"))
  (:`Pressed`
    (bind _running (`self.DirectionBehaviour` "NewEnumerator1"))
    (if _running
      (`KismetSystemLibrary.Delay` 0.2))))

(event `InputAction|Up`
  (params (Key :type "Key Structure"))
  (:`Pressed`
    (bind _running (`self.DirectionBehaviour` "NewEnumerator2"))
    (if _running
      (`KismetSystemLibrary.Delay` 0.2))))

(event `InputAction|Down`
  (params (Key :type "Key Structure"))
  (:`Pressed`
    (bind _running (`self.DirectionBehaviour` "NewEnumerator3"))
    (if _running
      (`KismetSystemLibrary.Delay` 0.2))))

(fn `DirectionBehaviour`
  (params (Direction :type "/Game/Data/ENUM_Direction Enum" :default "NewEnumerator0"))
  (returns (Running :type Boolean))
  (locals (IsRunning :type Boolean))
  (if (`local.IsRunning`)
    (set `local.IsRunning` true)
    (else
      (set `self.AnimationRunning` true)
      (bind _nextobject (`/Game/Blueprints/BP_Game.ShootTrace` (`self.CurrentGame`) Direction))
      (`self.SetNextGame` _nextobject)
      (bind _output_get (set `self.AnimationRunning` false))
      (set `local.IsRunning` _output_get)))
  (return (`local.IsRunning`)))

(fn `GetGames`
  (bind _outactors (`GameplayStatics.GetAllActorsOfClass` "/Game/Blueprints/BP_Game.BP_Game_C"))
  (set `self.ShownGames` _outactors))

(fn `GetProcessTracker`
  (bind _outactors (`GameplayStatics.GetAllActorsOfClass` "/Game/Blueprints/BP_ProcessTracker.BP_ProcessTracker_C"))
  (set `self.ProcessTracker` (`|GetArrayItem` _outactors)))

(fn `InitGames`
  (bind _asbp_game (cast `/Game/Blueprints/BP_Game` (`ChildActorComponent.ChildActor` (`self.0,0`))))
  (set `self.CurrentGame` _asbp_game)
  (for (_array_element _array_index) (`self.ShownGames`)
    (bind (_output_material _output_name) (break `/Game/Data/STRUCT_GameProperties` (`|GetArrayItem` (`self.YoungGames`) _array_index)))
    (`/Game/Blueprints/BP_Game.SetNewProperties` _array_element _output_material _output_name)))

(fn `SetNextGame`
  (params (Game :type "/Game/Blueprints/BP_Game Object Reference"))
  (`/Engine/EditorBlueprintResources/StandardMacros.IsValid` Game
    (:`Is Valid`
      (set `self.CurrentGame` Game))))

(fn `UserConstructionScript`)